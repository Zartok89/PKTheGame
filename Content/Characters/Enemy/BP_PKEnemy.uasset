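; BP_PKEnemy is an enemy character that takes damage and is destroyed when its health runs out.
; Health starts at MaxHealth on BeginPlay, and each AnyDamage event subtracts from it and prints the remaining value.
; A Healthbar widget component's UI_LifeBar progress bar then updates to the current health ratio before the actor destroys itself at zero.
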(event EventBeginPlay
  (Variables|Default|SetCurrentHealth (Variables|Default|GetMaxHealth)))

(event Game|Damage|EventAnyDamage
  (params (Damage :type Float%20%28single-precision%29) (DamageType :type Damage%20Type%20Object%20Reference) (InstigatedBy :type Controller%20Object%20Reference) (DamageCauser :type Actor%20Object%20Reference))
  (if (> (Variables|Default|GetCurrentHealth) 0.0)
    (bind _output_get (Variables|Default|SetCurrentHealth (- (Variables|Default|GetCurrentHealth) Damage)))
    (Development|PrintString (Utilities|String|ToString(Float) _output_get))
    (bind _asui_life_bar (Utilities|Casting|CastToUI_LifeBar (UserInterface|GetWidget (Variables|Default|GetHealthbar))))
    (Progress|SetPercent (Variables|/Game/TEMP/Variant_Combat/UI/UI_LifeBar.UI_LifeBar_C|GetBar _asui_life_bar) (Math|Float|SafeDivide (Variables|Default|GetCurrentHealth) (Variables|Default|GetMaxHealth)))
    (if (<= (Variables|Default|GetCurrentHealth) 0.0)
      (Actor|DestroyActor))))

(fn ConstructionScript)